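; BP_ClockManager is a manager that spawns clocks and listens for their alerts.
; On BeginPlay it spawns three BP_Clock actors at random heights, then binds one handler to the OnClockAlert dispatcher of every BP_Clock in the level.
; The handler prints the Cuckoo value passed by the alert to the screen as debug text.
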(event `self.ReceiveBeginPlay`
  (`|ExecutionSequence`
    (:`then_0`
      (for _ (range 1 4)
        (`|SpawnActorFromClass` "/Game/Blueprints/BP_Clock.BP_Clock_C" (`KismetMathLibrary.MakeTransform` (`KismetMathLibrary.MakeVector` 0.0 0.0 (`KismetMathLibrary.RandomFloatInRange` 0.0 1000.0))) "AlwaysSpawn" "MultiplyWithRoot" null null)))
    (:`then_1`
      ;[0 0.1211 0.15 0.5] register clocks to alert event
      (bind _outactors (`GameplayStatics.GetAllActorsOfClass` "/Game/Blueprints/BP_Clock.BP_Clock_C"))
      (for _array_element _outactors
        (add `/Game/Blueprints/BP_Clock.OnClockAlert` _array_element (delegate `OnClockAlert_Event`))))))

(event `OnClockAlert_Event`
  (params (Cuckoo :type Boolean))
  (`KismetSystemLibrary.PrintString` (`KismetStringLibrary.Concat_StrStr` "clock =" (`KismetStringLibrary.Conv_BoolToString` Cuckoo))))

(fn `UserConstructionScript`)