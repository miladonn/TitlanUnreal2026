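; BP_MoveableCube is a test actor that raises its static mesh steadily along relative Z.
; Tick adds a fixed, frame-rate-dependent offset without sweep, then prints the mesh's world location under a single message key.
; Leftover unconnected nodes for debug printing and a delayed hide/show of the mesh never run, and the construction script is empty.
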(event `self.ReceiveTick`
  (params (DeltaSeconds :type "Float (single-precision)"))
  (bind _staticmeshcomponent (`StaticMeshActor.StaticMeshComponent` ""))
  (`SceneComponent.K2_AddRelativeLocation` _staticmeshcomponent (0.0 0.0 1.0) false false)
  (`KismetSystemLibrary.PrintString` (`KismetStringLibrary.Conv_VectorToString` (`SceneComponent.K2_GetComponentLocation` _staticmeshcomponent)) true true (struct :`G` 0.66 :`B` 1.0 :`A` 1.0) 2.0 "Location"))

(fn `UserConstructionScript`)