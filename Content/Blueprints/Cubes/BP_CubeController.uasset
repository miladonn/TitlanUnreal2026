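; BP_CubeController triggers the upward movement of all BP_NewCube actors in the level after a configurable delay.
; On BeginPlay it collects the cubes, waits for DelayBeforeMove, then calls MoveUpEvent on each one still valid.
; It also casts each to BP_NewCube_Child to set ChildVar, printing a message when the cast fails.
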(event `self.ReceiveBeginPlay`
  ;[0.15 0 0.112 0.5] Move all the cubes upward
  (bind _outactors (`GameplayStatics.GetAllActorsOfClass` "/Game/Blueprints/Cubes/BP_NewCube.BP_NewCube_C"))
  (bind _output_get (set `self.Out Actors` _outactors))
  (`KismetSystemLibrary.Delay` (`self.DelayBeforeMove`))
  ;;[0 0.01113 0.15 0.5] The inner loop
  (for _array_element _output_get
    (`/Engine/EditorBlueprintResources/StandardMacros.IsValid` _array_element
      (:`Is Valid`
        (`/Game/Blueprints/Cubes/BP_NewCube.MoveUpEvent` _array_element)
        (bind _asbp_new_cube_child (cast `/Game/Blueprints/Cubes/BP_NewCube_Child` _array_element)
          (:`then`
            (set `/Game/Blueprints/Cubes/BP_NewCube_Child.ChildVar` true _asbp_new_cube_child))
          (:`CastFailed`
            (`KismetSystemLibrary.PrintString` "Can not cast to cube child!")))))))

(fn `UserConstructionScript`)