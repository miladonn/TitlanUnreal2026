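; BP_CubeController is a controller Blueprint that sets every BP_NewCube in the level moving shortly after play begins.
; On BeginPlay it gathers all cube actors, waits DelayBeforeMove, then calls MoveUpEvent on each one that is still valid.
; Disconnected leftover nodes for finding a single cube and setting its CanMove flag never run.
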(event `self.ReceiveBeginPlay`
  (bind _outactors (`GameplayStatics.GetAllActorsOfClass` "/Game/Blueprints/BP_NewCube.BP_NewCube_C"))
  (bind _output_get (set `self.Out Actors` _outactors))
  (`KismetSystemLibrary.Delay` (`self.DelayBeforeMove`))
  (for _array_element _output_get
    (`/Engine/EditorBlueprintResources/StandardMacros.IsValid` _array_element
      (:`Is Valid`
        (`/Game/Blueprints/BP_NewCube.MoveUpEvent` _array_element)))))

(fn `UserConstructionScript`)